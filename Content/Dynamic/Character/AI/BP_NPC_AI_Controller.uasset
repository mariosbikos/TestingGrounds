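; AI controller for NPCs that starts the patrol blackboard and guard behavior tree on BeginPlay.
; Perception updates feed the blackboard's EnemyKey for any perceived actor without the "Enemy" tag.
; A successful sense stores player pawn 0 in that key rather than the perceived actor, and a failed sense clears it.
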(event OnTargetPerceptionUpdated(AIPerception)
  (params (Actor :type Actor%20Object%20Reference) (Stimulus :type AI%20Stimulus%20Structure))
  (CallFunction|UpdateBlackboardEnemyKey (stale EventBeginPlay _blackboardcomponent) (stale EventBeginPlay _blackboardcomponent) Actor Stimulus))

(event EventBeginPlay
  (bind _blackboardcomponent (Class|AIController|UseBlackboard "/Game/Dynamic/Character/AI/BB_Patrol.BB_Patrol"))
  (AI|RunBehaviorTree "/Game/Dynamic/Character/AI/BT_GuardBehavior.BT_GuardBehavior"))

(fn ConstructionScript)

(fn UpdateBlackboardEnemyKey
  (params (self2 :type Blackboard%20Component%20Object%20Reference) (self3 :type Blackboard%20Component%20Object%20Reference) (self4 :type Actor%20Object%20Reference) (AIStimulus :type AI%20Stimulus%20Structure%20%28by%20ref%29))
  (bind _enemykey (Variables|Default|GetEnemyKey))
  (if (not (Actor|ActorHasTag self4 "Enemy"))
    (if (.bSuccessfullySensed (Utilities|Struct|BreakAIStimulus AIStimulus))
      (AI|Components|Blackboard|SetValueasObject self2 _enemykey (Game|Player|GetPlayerPawn 0))
      (else
        (AI|Components|Blackboard|ClearValue self3 _enemykey)))))