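; BP_Tile is one segment of the infinite terrain, scattering containers, boxes, rocks and cannisters in random counts through PlaceActors on BeginPlay.
; Its barrier starts locked, opens while the player overlaps LockingVolume, then relocks on exit and asks BP_InfiniteTerrainGameMode to spawn another tile.
; GetAttachLocation exposes the Arrow transform as an attach point, and the tile destroys itself when the player enters DestroyVolume.
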(event OnComponentBeginOverlap(LockingVolume)
  (params (OverlappedComponent :type Primitive%20Component%20Object%20Reference) (OtherActor :type Actor%20Object%20Reference) (OtherComp :type Primitive%20Component%20Object%20Reference) (OtherBodyIndex :type Integer) (bFromSweep :type Boolean) (SweepResult :type Hit%20Result%20Structure%20%28by%20ref%29))
  (Utilities|IsPlayerActor OtherActor)
  (CallFunction|Unlock))

(event OnComponentEndOverlap(LockingVolume)
  (params (OverlappedComponent :type Primitive%20Component%20Object%20Reference) (OtherActor :type Actor%20Object%20Reference) (OtherComp :type Primitive%20Component%20Object%20Reference) (OtherBodyIndex :type Integer))
  (Utilities|IsPlayerActor OtherActor)
  (CallFunction|Lock)
  (bind _asbp_infinite_terrain_game_mode (Utilities|Casting|CastToBP_InfiniteTerrainGameMode (Game|GetGameMode)))
  (Default|SpawnTile _asbp_infinite_terrain_game_mode))

(event OnComponentBeginOverlap(DestroyVolume)
  (params (OverlappedComponent :type Primitive%20Component%20Object%20Reference) (OtherActor :type Actor%20Object%20Reference) (OtherComp :type Primitive%20Component%20Object%20Reference) (OtherBodyIndex :type Integer) (bFromSweep :type Boolean) (SweepResult :type Hit%20Result%20Structure%20%28by%20ref%29))
  (Utilities|IsPlayerActor OtherActor)
  (Actor|DestroyActor))

(event EventBeginPlay
  (CallFunction|Lock)
  (Class|Tile|PlaceActors "/Game/Dynamic/Terrain/Props/BP_Container.BP_Container_C" 2 5)
  (Class|Tile|PlaceActors "/Game/Dynamic/Terrain/Props/BP_Box.BP_Box_C" 1 5)
  (Class|Tile|PlaceActors "/Game/Dynamic/Terrain/Props/BP_Rock.BP_Rock_C" 2 6)
  (Class|Tile|PlaceActors "/Game/Dynamic/Terrain/Props/BP_Cannister.BP_Cannister_C" 2 3))

(fn ConstructionScript)

(fn GetAttachLocation
  (return (Transformation|GetWorldTransform (Variables|Default|GetArrow))))

(fn Lock
  (bind _barrier (Variables|Default|GetBarrier))
  (Collision|SetCollisionEnabled _barrier "QueryAndPhysics")
  (Rendering|Material|SetMaterial _barrier 0 "/Game/Static/Geometry/Meshes/Barrier_Locked.Barrier_Locked"))

(fn Unlock
  (bind _barrier (Variables|Default|GetBarrier))
  (Collision|SetCollisionEnabled _barrier "NoCollision")
  (Rendering|Material|SetMaterial _barrier 0 "/Game/Static/Geometry/Meshes/Barrier_Unlocked.Barrier_Unlocked"))